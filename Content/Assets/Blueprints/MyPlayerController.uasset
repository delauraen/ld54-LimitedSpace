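; Player controller that handles movement, look and pause input for the third-person character.
; BeginPlay caches the player character as MyChar, and axis events feed it movement along its actor forward and right vectors plus pitch and yaw.
; Pause clears all widgets, then toggles game pause, showing either the character's pause menu or its HUD.
; A jump call is present but unconnected, so it never runs.
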(event `InputAction|Pause` :paused true
  (params (Key :type "Key Structure"))
  ;[1 1 1] Pause Game
  (:`Pressed`
    (`WidgetLayoutLibrary.RemoveAllWidgets`)
    (if (`GameplayStatics.IsGamePaused`)
      (`UserWidget.AddToViewport` (`/Game/ThirdPerson/Blueprints/BP_ThirdPersonCharacter.MyHUD` (`self.MyChar`)) 0)
      (`GameplayStatics.SetGamePaused` false)
      (else
        (`UserWidget.AddToViewport` (`/Game/ThirdPerson/Blueprints/BP_ThirdPersonCharacter.PauseMenu` (`self.MyChar`)) 0)
        (`GameplayStatics.SetGamePaused` true)))))

(event `InputAxis|MoveForwardBack`
  (params (AxisValue :type "Float (single-precision)"))
  (bind _mychar (`self.MyChar`))
  ;[1 1 1] Character Movement
  (`Pawn.AddMovementInput` _mychar (`self.GetActorForwardVector` _mychar) AxisValue false))

(event `InputAxis|LookUpDown`
  (params (AxisValue :type "Float (single-precision)"))
  ;[1 1 1] Character Look Around
  (`Pawn.AddControllerPitchInput` (`self.MyChar`) AxisValue))

(event `InputAxis|MoveLeftRight`
  (params (AxisValue :type "Float (single-precision)"))
  (bind _mychar (`self.MyChar`))
  ;[1 1 1] Character Movement
  (`Pawn.AddMovementInput` _mychar (`self.GetActorRightVector` _mychar) AxisValue false))

(event `InputAxis|LookLeftRight`
  (params (AxisValue :type "Float (single-precision)"))
  ;[1 1 1] Character Look Around
  (`Pawn.AddControllerYawInput` (`self.MyChar`) AxisValue))

(event `self.ReceiveBeginPlay`
  (bind _asbp_third_person_character (cast `/Game/ThirdPerson/Blueprints/BP_ThirdPersonCharacter` (`GameplayStatics.GetPlayerCharacter` 0)))
  (set `self.MyChar` _asbp_third_person_character))

(fn `UserConstructionScript`)