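; Goose enemy that steals a grocery bag from the third-person player when they touch its capsule while holding one.
; On overlap it detaches a random overlapping GroceryBag and the character from their parents, spawns a new bag at GooseSocket, honks and decrements the player's BagsCollected.
; An EnemyMovement timeline that lerps the goose to EndingLocation is present but never triggered.
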(event `self.Capsule.OnComponentBeginOverlap`
  (params (OverlappedComponent :type "PrimitiveComponent Object Reference") (OtherActor :type "Actor Object Reference") (OtherComp :type "PrimitiveComponent Object Reference") (OtherBodyIndex :type Integer) (bFromSweep :type Boolean) (SweepResult :type "HitResult Structure (by ref)"))
  (bind _asbp_third_person_character (cast `/Game/ThirdPerson/Blueprints/BP_ThirdPersonCharacter` OtherActor))
  (if (`/Game/ThirdPerson/Blueprints/BP_ThirdPersonCharacter.IsHolding` _asbp_third_person_character)
    (`KismetSystemLibrary.PrintString` "goose steal!")
    (`self.K2_DetachFromActor` (`KismetArrayLibrary.Array_Random` (`PrimitiveComponent.GetOverlappingActors` (`self.Capsule`) "/Game/Assets/Blueprints/GroceryBag.GroceryBag_C")) "KeepRelative" "KeepRelative" "KeepRelative")
    (`self.K2_DetachFromActor` _asbp_third_person_character "KeepRelative" "KeepRelative" "KeepRelative")
    (`|SpawnActorFromClass` "/Game/Assets/Blueprints/GroceryBag.GroceryBag_C" (`SceneComponent.GetSocketTransform` (`self.Goose`) "GooseSocket" "RTS_World") "Undefined" "MultiplyWithRoot" null null)
    (`GameplayStatics.PlaySound2D` "/Game/Assets/Sound/honk-sound.honk-sound" 1.0 1.0 0.0 null null)
    (bind _asbp_third_person_character_2 (cast `/Game/ThirdPerson/Blueprints/BP_ThirdPersonCharacter` OtherActor))
    (set `/Game/ThirdPerson/Blueprints/BP_ThirdPersonCharacter.BagsCollected` (- (`/Game/ThirdPerson/Blueprints/BP_ThirdPersonCharacter.BagsCollected` _asbp_third_person_character_2) 1) _asbp_third_person_character_2)))

(fn `UserConstructionScript`)